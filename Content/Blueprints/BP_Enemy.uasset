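; BP_Enemy is a melee enemy that chases the player and knocks them back with a crowbar attack.
; Each PawnSensing sighting starts an AI move toward the player, and arrival plays the attack montage, gated by CanAttack until it completes or is interrupted.
; A montage notify fires a short forward sphere trace with debug drawing, launching any hit Character forward and upward without applying damage.
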(event OnSeePawn(PawnSensing)
  (params (Pawn :type Pawn%20Object%20Reference))
  (CallFunction|ChasePlayer))

(event Custom|Chase%20Player
  (bind _returnvalue (Transformation|GetActorLocation))
  (AI|AIMoveTo self "0, 0, 0" (Game|GetPlayerCharacter 0) 1.2e+02 false
    (:OnSuccess
      (if (Variables|Default|GetCanAttack)
        (Animation|Montage|PlayMontage (Variables|Character|GetMesh) "/Game/ST_Characters_JC/Animation/Attack/A_Crowbar_Attack_Montage.A_Crowbar_Attack_Montage"
          (:then
            (Variables|Default|SetCanAttack false))
          (:OnCompleted
            (Variables|Default|SetCanAttack true :!label _label))
          (:OnInterrupted
            (goto _label))
          (:OnNotifyBegin
            (bind (_outhit _returnvalue_2) (Collision|SphereTraceByChannel _returnvalue (+ _returnvalue (* (Math|Vector|GetForwardVector (Transformation|GetActorRotation)) 1.2e+02)) 25.0 "TraceTypeQuery3" false 0 "ForDuration" true "(R=1.000000,G=0.000000,B=0.000000,A=1.000000)" "(R=0.000000,G=1.000000,B=0.000000,A=1.000000)" 0.5))
            (if _returnvalue_2
              (bind _as角色 (Utilities|Casting|CastToCharacter (.HitActor (Collision|BreakHitResult _outhit))))
              (Character|LaunchCharacter _as角色 (+ (* (Math|Vector|GetForwardVector (Transformation|GetActorRotation)) (Variables|Default|GetfrontalKnockBar)) (Math|Vector|MakeVector 0.0 0.0 (Variables|Default|GetUpwardsKnockBar))) false false))))))))

(event EventBeginPlay)

(event Collision|EventActorBeginOverlap
  (params (OtherActor :type Actor%20Object%20Reference)))

(event EventTick
  (params (DeltaSeconds :type Float%20%28single-precision%29)))

(fn ConstructionScript)